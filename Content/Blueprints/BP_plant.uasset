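; BP_plant turns a viewer's Kinect-tracked movement into an interactive plant's bend and bloom.
; Each tick, the nearest body's SpineBase Y sets bend and Z sets bloom, from bud when near to flower when far.
; Clamped values ease via FInterpTo with fixed delta times, drifting back to upright, open bloom when nobody is detected.
; Results are written to BP_Controller's BowDegree and Blooming; the sensor lives from BeginPlay to EndPlay.
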(event Custom|人的运动控制植物形态
  (bind (_hasbody _returnvalue) (Class|NeoKinectManager|GetNearestBody))
  (bind _returnvalue_2 (Class|NeoKinectBody|GetJointLocation _returnvalue "SpineBase"))
  (bind (_x _y _z) (Math|Vector|BreakVector _returnvalue_2))
  (if (Class|NeoKinectManager|IsKinectAvailable)
    (if _hasbody
      ;[1 1 1] 有人
      (Utilities|FlowControl|Sequence
        (:then_0
          ;;[1 1 1] y位置-100（右）到100（左）之间，控制弯腰幅度
          (bind _output_get (Variables|Default|SetBow (Math|Interpolation|FInterpTo (Variables|Default|GetBow) (Math|Float|Clamp(Float) _y -1e+02 1e+02) 0.1 0.2))))
        (:then_1
          ;;[1 1 1] 距离近是花骨朵，远了是花，范围[-25远,-10近]
          (bind _output_get_2 (Variables|Default|SetBloom (Math|Interpolation|FInterpTo (Variables|Default|GetBloom) (Math|Float|Clamp(Float) _z -25.0 -1e+01) 0.1 0.2))))
        (:then_2
          ;;[1 1 1] 数据传输
          (bind _asbp_controller (Utilities|Casting|CastToBP_Controller (Game|GetPlayerController 0)))
          (Variables|/Game/Blueprints/BP_Controller.BP_Controller_C|SetBow%20Degree _asbp_controller (Variables|Default|GetBow)))
        (:then_3
          (bind _asbp_controller_2 (Utilities|Casting|CastToBP_Controller (Game|GetPlayerController 0)))
          (Variables|/Game/Blueprints/BP_Controller.BP_Controller_C|SetBlooming _asbp_controller_2 (Variables|Default|GetBloom))))
      (else
        ;[1 1 1] 无人
        (Utilities|FlowControl|Sequence
          (:then_0
            ;;[1 1 1] 无人时慢慢回复开花直立状态
            (Variables|Default|SetBow (Math|Interpolation|FInterpTo (Variables|Default|GetBow) 0.0 0.05 0.2))
            (Variables|Default|SetBloom (Math|Interpolation|FInterpTo (Variables|Default|GetBloom) -25.0 0.05 0.2)))
          (:then_1
            ;;[1 1 1] 数据传输
            (bind _asbp_controller_3 (Utilities|Casting|CastToBP_Controller (Game|GetPlayerController 0)))
            (Variables|/Game/Blueprints/BP_Controller.BP_Controller_C|SetBow%20Degree _asbp_controller_3 (Variables|Default|GetBow)))
          (:then_2
            (bind _asbp_controller_4 (Utilities|Casting|CastToBP_Controller (Game|GetPlayerController 0)))
            (Variables|/Game/Blueprints/BP_Controller.BP_Controller_C|SetBlooming _asbp_controller_4 (Variables|Default|GetBloom))))))))

(event EventBeginPlay
  (Class|NeoKinectManager|InitSensor))

(event EventTick
  (params (DeltaSeconds :type Float%20%28single-precision%29))
  (CallFunction|人的运动控制植物形态))

(event EventEndPlay
  (params (EndPlayReason :type EEndPlayReason%20Enum :default "Destroyed"))
  (Class|NeoKinectManager|UninitSensor))

(fn ConstructionScript)